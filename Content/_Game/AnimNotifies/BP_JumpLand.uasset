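; BP_JumpLand is an animation notify that plays a jump landing sound for the shooter character, matched to the ground surface.
; It casts the mesh owner to BP_ShooterCharacter, reads its surface type and selects the metal, stone, tile, grass or water cue, with stone as the fallback.
; The chosen cue plays at the owning actor's location; other owner types play nothing.
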(fn ReceivedNotify
  (params (MeshComp :type Skeletal%20Mesh%20Component%20Object%20Reference) (Animation :type Anim%20Sequence%20Base%20Object%20Reference) (EventReference :type Anim%20Notify%20Event%20Reference%20Structure%20%28by%20ref%29))
  (bind _returnvalue (Components|GetOwner MeshComp))
  (bind _asbp_shooter_character (Utilities|Casting|CastToBP_ShooterCharacter _returnvalue))
  (bind _returnvalue_2 (Class|ShooterCharacter|GetSurfaceType _asbp_shooter_character))
  (switch Utilities|FlowControl|Switch|SwitchonEPhysicalSurface _returnvalue_2
    (:SurfaceType_Default
      (LocalVariables|SetLandingSound "/Game/_Game/Assets/Sounds/Footsteps/Stone/JumpLand_Stone_Cue.JumpLand_Stone_Cue"))
    (:SurfaceType1
      (LocalVariables|SetLandingSound "/Game/_Game/Assets/Sounds/Footsteps/Metal/JumpLand_Metal_Cue.JumpLand_Metal_Cue"))
    (:SurfaceType2
      (LocalVariables|SetLandingSound "/Game/_Game/Assets/Sounds/Footsteps/Stone/JumpLand_Stone_Cue.JumpLand_Stone_Cue"))
    (:SurfaceType3
      (LocalVariables|SetLandingSound "/Game/_Game/Assets/Sounds/Footsteps/Tile/JumpLand_Tile_Cue.JumpLand_Tile_Cue"))
    (:SurfaceType4
      (LocalVariables|SetLandingSound "/Game/_Game/Assets/Sounds/Footsteps/Grass/JumpLand_Grass_Cue.JumpLand_Grass_Cue"))
    (:SurfaceType5
      (LocalVariables|SetLandingSound "/Game/_Game/Assets/Sounds/Footsteps/Water/JumpLand_Water_Cue.JumpLand_Water_Cue")))
  (Audio|PlaySoundatLocation (LocalVariables|GetLandingSound) (Transformation|GetActorLocation _returnvalue) "0, 0, 0" 1.0 1.0 0.0 0 0 0 0)
  (return false))