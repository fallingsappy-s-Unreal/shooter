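; Footstep anim notify that plays surface-dependent sound and Niagara effects for BP_ShooterCharacter, and does nothing for other mesh owners.
; It switches on the character's GetSurfaceType to pick a sound and particle pair for metal, stone, tile, grass, water or a default.
; A shared helper spawns both at the BoneName socket, with ShouldPlaySound gating only the sound, so particles always spawn.
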(fn ReceivedNotify
  (params (MeshComp :type Skeletal%20Mesh%20Component%20Object%20Reference) (Animation :type Anim%20Sequence%20Base%20Object%20Reference) (EventReference :type Anim%20Notify%20Event%20Reference%20Structure%20%28by%20ref%29))
  (LocalVariables|SetMesh%20Comp MeshComp)
  (bind _asbp_shooter_character (Utilities|Casting|CastToBP_ShooterCharacter (Components|GetOwner MeshComp)))
  (bind _returnvalue (Class|ShooterCharacter|GetSurfaceType _asbp_shooter_character))
  (switch Utilities|FlowControl|Switch|SwitchonEPhysicalSurface _returnvalue
    (:SurfaceType_Default
      (CallFunction|PlaySoundandSpawnParticles "/Game/_Game/Assets/Sounds/Footsteps/Rock/FootstepRock_Cue.FootstepRock_Cue" "/Game/A_Surface_Footstep/Niagara_FX/ParticleSystems/PSN_General1_Surface.PSN_General1_Surface" (LocalVariables|GetMesh%20Comp)))
    (:SurfaceType1
      (CallFunction|PlaySoundandSpawnParticles "/Game/_Game/Assets/Sounds/Footsteps/Metal/FootstepMetal_Cue.FootstepMetal_Cue" "/Game/A_Surface_Footstep/Niagara_FX/ParticleSystems/PSN_General1_Surface.PSN_General1_Surface" (LocalVariables|GetMesh%20Comp)))
    (:SurfaceType2
      (CallFunction|PlaySoundandSpawnParticles "/Game/_Game/Assets/Sounds/Footsteps/Rock/FootstepRock_Cue.FootstepRock_Cue" "/Game/A_Surface_Footstep/Niagara_FX/ParticleSystems/PSN_Gravel_Surface.PSN_Gravel_Surface" (LocalVariables|GetMesh%20Comp)))
    (:SurfaceType3
      (CallFunction|PlaySoundandSpawnParticles "/Game/_Game/Assets/Sounds/Footsteps/Tile/FootstepTile_Cue.FootstepTile_Cue" "/Game/A_Surface_Footstep/Niagara_FX/ParticleSystems/PSN_General2_Surface.PSN_General2_Surface" (LocalVariables|GetMesh%20Comp)))
    (:SurfaceType4
      (CallFunction|PlaySoundandSpawnParticles "/Game/_Game/Assets/Sounds/Footsteps/Grass/FootstepGrass_Cue.FootstepGrass_Cue" "/Game/A_Surface_Footstep/Niagara_FX/ParticleSystems/PSN_Grass_Surface.PSN_Grass_Surface" (LocalVariables|GetMesh%20Comp)))
    (:SurfaceType5
      (CallFunction|PlaySoundandSpawnParticles "/Game/_Game/Assets/Sounds/Footsteps/Water/FootstepWater_Cue.FootstepWater_Cue" "/Game/A_Surface_Footstep/Niagara_FX/ParticleSystems/PSN_WaterLight_Surface.PSN_WaterLight_Surface" (LocalVariables|GetMesh%20Comp))))
  (return false))

(fn PlaySoundandSpawnParticles
  (params (Sound :type Sound%20Base%20Object%20Reference) (Particles :type Niagara%20System%20Object%20Reference) (MeshComp :type Skeletal%20Mesh%20Component%20Object%20Reference))
  (bind _bonename (Variables|Default|GetBoneName))
  (bind _returnvalue (Transformation|GetSocketLocation MeshComp _bonename))
  (if (Variables|Default|GetShouldPlaySound)
    (Audio|PlaySoundatLocation Sound _returnvalue "0, 0, 0" 1.0 1.0 0.0 0 0 0 0))
  (Niagara|SpawnSystematLocation Particles _returnvalue))