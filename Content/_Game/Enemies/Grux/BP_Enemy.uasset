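; BP_Enemy is an enemy Blueprint that drives the enemy's health bar and on-hit damage numbers.
; On BeginPlay it links the health bar widget to itself and starts it hidden, with events to show and hide it.
; Each hit spawns an animated number widget, flagged for headshots, at the hit location projected to screen space.
; The widget and world location are then handed to StoreHitNumber.
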(event EventBeginPlay
  (bind _asbp_enemy_health_bar (Utilities|Casting|CastToBP_EnemyHealthBar (UserInterface|GetUserWidgetObject (Variables|Default|GetHealthBar))))
  (Variables|/Game/_Game/HUD/BP_EnemyHealthBar.BP_EnemyHealthBar_C|SetEnemy _asbp_enemy_health_bar self)
  (Widget|SetVisibility _asbp_enemy_health_bar "Hidden"))

(event EventShowHitNumber
  (params (Damage :type Integer) (HitLocation :type Vector :default "0, 0, 0") (bHeadShot :type Boolean))
  (Variables|Default|SetHead%20Shot bHeadShot)
  (bind _returnvalue (UserInterface|CreateWidget "/Game/_Game/HUD/BP_HitNumber.BP_HitNumber_C"))
  (Variables|Default|SetHitNumberWidget _returnvalue)
  (Variables|/Game/_Game/HUD/BP_HitNumber.BP_HitNumber_C|SetHitText (Variables|Default|GetHitNumberWidget) (Utilities|Text|ToText(Integer) Damage))
  (UserInterface|Animation|PlayAnimation (Variables|Default|GetHitNumberWidget) (Variables|/Game/_Game/HUD/BP_HitNumber.BP_HitNumber_C|GetHitNumberAnimation (Variables|Default|GetHitNumberWidget)) 0.0 1 "Forward" 1.0 false)
  (Variables|/Game/_Game/HUD/BP_HitNumber.BP_HitNumber_C|SetHeadShot (Variables|Default|GetHitNumberWidget) (Variables|Default|GetHead%20Shot))
  (UserInterface|Viewport|AddtoViewport (Variables|Default|GetHitNumberWidget) 0)
  (Class|UserWidget|SetPositioninViewport (Variables|Default|GetHitNumberWidget) (.ScreenPosition (Class|GameplayStatics|ProjectWorldtoScreen (Game|GetPlayerController 0) HitLocation false)) true)
  (Class|Enemy|StoreHitNumber (Variables|Default|GetHitNumberWidget) HitLocation))

(event EventShowHealthBar
  (Widget|SetVisibility (UserInterface|GetUserWidgetObject (Variables|Default|GetHealthBar)) "Visible")
  (|CallParentFunction))

(event EventHideHealthBar
  (Widget|SetVisibility (UserInterface|GetUserWidgetObject (Variables|Default|GetHealthBar)) "Hidden"))

(fn ConstructionScript)